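; BP_OpenDriveReader reads OpenDRIVE road-network coordinates from its OpenDrive object and stores them in its own variables.
; The construction script copies road ID, lane ID, S, T, H and junction ID, so values update only when construction reruns.
; A GetPosition call is wired into that chain but never executes, and the event graph holds only empty, disabled default events.
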(fn `UserConstructionScript`
  (set `self.Road Id` (`OpenDriveComponent.GetRoadId` (`self.OpenDrive`)))
  (set `self.Lane Id` (`OpenDriveComponent.GetLaneId` (`self.OpenDrive`)))
  (set `self.S` (`OpenDriveComponent.GetS` (`self.OpenDrive`)))
  (set `self.T` (`OpenDriveComponent.GetT` (`self.OpenDrive`)))
  (set `self.H` (`OpenDriveComponent.GetH` (`self.OpenDrive`)))
  (set `self.Junction Id` (`OpenDriveComponent.GetJunctionId` (`self.OpenDrive`))))
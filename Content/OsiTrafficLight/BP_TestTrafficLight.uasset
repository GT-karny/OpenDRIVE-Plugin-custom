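; Test traffic light actor that displays red, yellow and green lamp states by recoloring its meshes.
; The construction script creates a dynamic M_Light material instance for each lamp.
; The state-changed event passes color and mode to TrafficLightUpdate, which switches that lamp's BaseColor between its color and black.
; Only Off and Constant modes are handled, and each update affects a single lamp.
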(event `self.ReceiveTick`
  (params (DeltaSeconds :type "Float (single-precision)")))

(event `self.OnTrafficLightStateChanged`
  (params (NewState :type "OsiTrafficLightState Structure (by ref)"))
  (`self.Traffic Light Update` NewState_Color NewState_Mode))

(fn `Traffic Light Update`
  (params (InputPin :type "EOsiTrafficLightColor Enum" :default "UNKNOWN") (InputPin2 :type "EOsiTrafficLightMode Enum" :default "UNKNOWN"))
  (locals (isOn :type Boolean))
  (bind _redmaterial (`self.RedMaterial`))
  (bind _ison (`local.isOn`))
  (bind _yellowmaterial (`self.YellowMaterial`))
  (bind _greenmaterial (`self.GreenMaterial`))
  (switch `EOsiTrafficLightMode` InputPin2
    (:`OFF`
      (set `local.isOn` false))
    (:`CONSTANT`
      (set `local.isOn` true)))
  (switch `EOsiTrafficLightColor` InputPin
    (:`RED`
      (set `self.isRed` _ison)
      (if (`self.isRed`)
        (`MaterialInstanceDynamic.SetVectorParameterValue` _redmaterial "BaseColor" (struct :`R` 1.0 :`A` 1.0))
        (else
          (`MaterialInstanceDynamic.SetVectorParameterValue` _redmaterial "BaseColor" (struct :`A` 1.0)))))
    (:`YELLOW`
      (set `self.isYellow` _ison)
      (if (`self.isYellow`)
        (`MaterialInstanceDynamic.SetVectorParameterValue` _yellowmaterial "BaseColor" (struct :`R` 1.0 :`G` 1.0 :`A` 1.0))
        (else
          (`MaterialInstanceDynamic.SetVectorParameterValue` _yellowmaterial "BaseColor" (struct :`A` 1.0)))))
    (:`GREEN`
      (set `self.isGreen` _ison)
      (if (`self.isGreen`)
        (`MaterialInstanceDynamic.SetVectorParameterValue` _greenmaterial "BaseColor" (struct :`G` 1.0 :`A` 1.0))
        (else
          (`MaterialInstanceDynamic.SetVectorParameterValue` _greenmaterial "BaseColor" (struct :`A` 1.0)))))))

(fn `UserConstructionScript`
  (bind _returnvalue (`PrimitiveComponent.CreateDynamicMaterialInstance` (`self.Red`) 0 "/Game/M_Light.M_Light" "None"))
  (set `self.RedMaterial` _returnvalue)
  (bind _returnvalue_2 (`PrimitiveComponent.CreateDynamicMaterialInstance` (`self.Yellow`) 0 "/Game/M_Light.M_Light" "None"))
  (set `self.YellowMaterial` _returnvalue_2)
  (bind _returnvalue_3 (`PrimitiveComponent.CreateDynamicMaterialInstance` (`self.Green`) 0 "/Game/M_Light.M_Light" "None"))
  (set `self.GreenMaterial` _returnvalue_3))